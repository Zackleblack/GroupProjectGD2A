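; BP_CubePlatform is a platform that endlessly vanishes and reappears on a timer.
; IsColorRed sets the starting phase, so red cubes start visible while the others start hidden, putting the two groups in opposite phases.
; Two custom events call each other after equal delays, toggling the Platform's visibility and collision.
; The initial hide on non-red cubes leaves collision unchanged.
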(event Custom|Cube%20Vanish%20True
  (bind _platform (Variables|Default|GetPlatform))
  ;[0.15 0.15 0.15 0.5] Cube Vanish Time
  (Utilities|FlowControl|Delay 4.0)
  (Utilities|FlowControl|Sequence
    (:then_0
      (Development|SetHiddeninGame _platform true false))
    (:then_1
      (Collision|SetCollisionEnabled _platform "NoCollision"))
    (:then_2
      (CallFunction|CubeVanishFalse))))

(event Custom|Cube%20Vanish%20False
  (bind _platform (Variables|Default|GetPlatform))
  ;[0.15 0.15 0.15 0.5] Cube Appear Time
  (Utilities|FlowControl|Delay 4.0)
  (Utilities|FlowControl|Sequence
    (:then_0
      (Development|SetHiddeninGame _platform false false))
    (:then_1
      (Collision|SetCollisionEnabled _platform "QueryAndPhysics"))
    (:then_2
      (CallFunction|CubeVanishTrue))))

(event EventBeginPlay
  ;[0.15 0.15 0.15 0.5] Decides what cube should vanish
  (if (Variables|Default|GetbIsColorRed?)
    (Utilities|FlowControl|Delay 0.3)
    (CallFunction|CubeVanishTrue)
    (else
      (Development|SetHiddeninGame (Variables|Default|GetPlatform) true false)
      (Utilities|FlowControl|Delay 0.3)
      (CallFunction|CubeVanishFalse))))

(fn ConstructionScript)