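; BP_CanonBall is a cannonball hazard that knocks the player character away and restarts the level on contact.
; Its collision overlap casts to BP_ZackThirdPersonCharacter and launches the character hard along the ball's forward vector.
; The camera then fades out, and a delayed console command restarts the level.
; BeginPlay calls CanonBallMoves, which is an empty event, so this graph does not move the ball.
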(event OnComponentBeginOverlap(CanonBallCollision)
  (params (OverlappedComponent :type Primitive%20Component%20Object%20Reference) (OtherActor :type Actor%20Object%20Reference) (OtherComp :type Primitive%20Component%20Object%20Reference) (OtherBodyIndex :type Integer) (bFromSweep :type Boolean) (SweepResult :type Hit%20Result%20Structure%20%28by%20ref%29))
  ;[0.15 0.15 0.15 0.5] Touching the Canon Ball launches the player and then restarts the level.
  (bind _asbp_zack_third_person_character (Utilities|Casting|CastToBP_ZackThirdPersonCharacter OtherActor) ; Geting Character to make sure this is what is hitting it.
    (:then
      (Development|PrintString "The character has been hit.")
      (Character|LaunchCharacter _asbp_zack_third_person_character (* (Math|Vector|GetForwardVector (Transformation|GetWorldRotation (Variables|Default|GetCanonBall))) 1.5e+04) false false)
      ;;[0.15 0.15 0.15 0.5] Player Coontroller is VERY IMPORTANT
      (CameraFades|StartCameraFade :self (Variables|/Script/Engine.PlayerController|GetPlayerCameraManager (Game|GetPlayerController 0)) :FromAlpha 0.0 :ToAlpha 1.0 :Duration 4.5 :bHoldWhenFinished true)
      (Utilities|FlowControl|Delay 5.0)
      (Development|ExecuteConsoleCommand "RestartLevel" 0))
    (:CastFailed
      (Development|PrintString "Not the Character"))))

(event Custom|CanonBall%20Moves)

(event EventBeginPlay
  (Utilities|FlowControl|Sequence
    (:then_0
      (CallFunction|CanonBallMoves))))

(event Collision|EventActorBeginOverlap
  (params (OtherActor :type Actor%20Object%20Reference)))

(event EventTick
  (params (DeltaSeconds :type Float%20%28single-precision%29)))

(fn ConstructionScript)