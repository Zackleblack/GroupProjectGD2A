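; BP_Launcher is an actor that spawns a BP_CanonBall at its Launcher component every three seconds, starting at BeginPlay.
; A self-calling custom event with a delay drives the repeating LaunchCanonBall event.
; Each spawned ball receives a velocity-change impulse, currently zero, so it gets no launch speed.
; A projectile velocity suggestion node is present but never runs.
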(event Custom|Launch%20Canon%20Ball
  (bind _returnvalue (Game|SpawnActorfromClass "/Game/Developer/Kaydyn/Blueprints/BP_CanonBall.BP_CanonBall_C" (Transformation|GetWorldTransform (Variables|Default|GetLauncher)) "Undefined" "MultiplyWithRoot" 0 0))
  (Physics|AddImpulse (Variables|/Game/Developer/Kaydyn/Blueprints/BP_CanonBall.BP_CanonBall_C|GetCanonBall _returnvalue) "0, 0, 0" "None" true))

(event Custom|CustomEvent
  (CallFunction|LaunchCanonBall)
  (Utilities|FlowControl|Delay 3.0)
  (CallFunction|CustomEvent))

(event EventBeginPlay
  (CallFunction|LaunchCanonBall)
  (Utilities|FlowControl|Delay 3.0)
  (CallFunction|CustomEvent))

(event Collision|EventActorBeginOverlap
  (params (OtherActor :type Actor%20Object%20Reference)))

(event EventTick
  (params (DeltaSeconds :type Float%20%28single-precision%29)))

(fn ConstructionScript)